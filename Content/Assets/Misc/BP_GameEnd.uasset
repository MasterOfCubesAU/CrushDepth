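; BP_GameEnd watches for the game-over condition and runs the ending sequence.
; Each Tick it reads submarine health and oxygen from GS_Core, triggering once when either hits zero.
; It plays an end sound and drives global time dilation from a slow-motion timeline, whose first update starts a camera shake.
; After a short delay, it shows the WB_GameEnd widget, enables the cursor and ignores move and look input.
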(event EventTick
  (params (DeltaSeconds :type Float%20%28single-precision%29))
  (bind _asgs_core (Utilities|Casting|CastToGS_Core (Game|GetGameState)))
  (bind _returnvalue (Class|GSCore|GetSubmarineHealth _asgs_core))
  (bind _returnvalue_2 (Class|GSCore|GetCurrentOxygen _asgs_core))
  (if (or (== _returnvalue_2 0.0) (== _returnvalue 0.0))
    (Utilities|FlowControl|DoOnce false
      (:Completed
        (Audio|PlaySound2D "/Game/Assets/Sounds/end_game.end_game" 1.0 1.0 0.0 0 0)
        (bind _newtrack_0 (Timeline|SlowMotionTimeline PlayFromStart)
          (:Update
            (Utilities|Time|SetGlobalTimeDilation _newtrack_0)
            (Utilities|FlowControl|DoOnce false
              (:Completed
                (Camera|PlayWorldCameraShake "/Game/Assets/Misc/BP_GameEndShake.BP_GameEndShake_C" (Transformation|GetActorLocation (Game|GetPlayerController 0)) 0.0 1.0 0.0)
                (Utilities|FlowControl|Delay 1.3)
                (CallFunction|CreateEndScreen)))))))))

(fn ConstructionScript)

(fn CreateEndScreen
  (bind _returnvalue (Game|GetPlayerController 0))
  (bind _returnvalue_2 (UserInterface|CreateWidget "/Game/UI/WB_GameEnd.WB_GameEnd_C" (Game|GetPlayerController 0)))
  (UserInterface|Viewport|AddtoViewport _returnvalue_2 0)
  (Input|SetInputModeGameandUI _returnvalue 0 "DoNotLock" true false)
  (Input|SetIgnoreMoveInput _returnvalue true)
  (Input|SetIgnoreLookInput _returnvalue true)
  (Variables|/Script/Engine.PlayerController|SetbShowMouseCursor _returnvalue true))
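; Tablet prop that displays the state of submarine systems and hull condition on text readouts.
; Every Tick it polls BP_TaskManager, marking each system's text ERROR or OK by whether its task is active.
; An active Broken Computer task instead spawns an attached BP_Broken_Tablet_Screen, found by world-wide class lookup and destroyed once the task clears.
; Hull text shows GOOD, MODERATE or CRITICAL from GS_Core's submarine health.
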(event EventTick
  (params (DeltaSeconds :type Float%20%28single-precision%29))
  (CallFunction|UpdateTaskStatus)
  (CallFunction|UpdateHullStatus))

(fn ConstructionScript)

(fn SetTaskStatus
  (params (TaskName :type String%20%28by%20ref%29) (TaskReference :type Text%203D%20Component%20Object%20Reference))
  (if (!= (Utilities|Array|FindItem (Variables|Default|GetActiveTasks) TaskName) -1)
    (Variables|/Script/Text3D.Text3DComponent|SetText TaskReference "ERROR")
    (else
      (Variables|/Script/Text3D.Text3DComponent|SetText TaskReference "OK"))))

(fn UpdateTaskStatus
  (bind _returnvalue (Actor|GetActorOfClass "/Game/Assets/Tasks/Templates/BP_TaskManager.BP_TaskManager_C"))
  (bind _tasknames (Default|GetTasks _returnvalue))
  (bind _output_get (Variables|Default|SetTaskList _tasknames))
  (bind _tasknames_2 (Default|GetActiveTasks _returnvalue))
  (Variables|Default|SetActiveTasks _tasknames_2)
  (for _array_element _output_get
    (switch string _array_element
      (:Broken%20Computer
        (Variables|Default|SetTaskIterator (Variables|Default|GetComputerStatus))
        (CallFunction|HandleComputerError))
      (:Engine%20Failure
        (Variables|Default|SetTaskIterator (Variables|Default|GetEngineStatus))
        (CallFunction|SetTaskStatus _array_element (Variables|Default|GetTaskIterator) :!label _label))
      (:Fire%20Outbreak
        (Variables|Default|SetTaskIterator (Variables|Default|GetFireStatus))
        (goto _label))
      (:Leak%20Task
        (Variables|Default|SetTaskIterator (Variables|Default|GetLeakStatus))
        (goto _label))
      (:Oxygen%20Failure
        (Variables|Default|SetTaskIterator (Variables|Default|GetOxygenStatus))
        (goto _label))
      (:Electrical%20Failure
        (Variables|Default|SetTaskIterator (Variables|Default|GetPowerStatus))
        (goto _label))
      (:Pressure%20Destabilising
        (Variables|Default|SetTaskIterator (Variables|Default|GetPressureStatus))
        (goto _label)))))

(fn UpdateHullStatus
  (bind _asgs_core (Utilities|Casting|CastToGS_Core (Game|GetGameState)))
  (bind _returnvalue (Class|GSCore|GetSubmarineHealth _asgs_core))
  (if (> _returnvalue 7e+01)
    (Variables|/Script/Text3D.Text3DComponent|SetText (Variables|Default|GetHullStatus) "GOOD")
    (elif (and (>= _returnvalue 2e+01) (<= _returnvalue 7e+01))
      (Variables|/Script/Text3D.Text3DComponent|SetText (Variables|Default|GetHullStatus) "MODERATE")
      (elif (< _returnvalue 2e+01)
        (Variables|/Script/Text3D.Text3DComponent|SetText (Variables|Default|GetHullStatus) "CRITICAL")))))

(fn CheckifNeedErrorScreen
  (bind _outactors (Actor|GetAllActorsOfClass "/Game/Assets/Props/TaskTablet/BP_Broken_Tablet_Screen.BP_Broken_Tablet_Screen_C"))
  (if (Utilities|Array|IsEmpty _outactors)
    (CallFunction|CreateErrorScreen)))

(fn CheckifNeedRemoveErrorScreen
  (bind _returnvalue (Actor|GetActorOfClass "/Game/Assets/Props/TaskTablet/BP_Broken_Tablet_Screen.BP_Broken_Tablet_Screen_C"))
  (if (Utilities|IsValid _returnvalue)
    (Actor|DestroyActor _returnvalue)))

(fn HandleComputerError
  (if (!= (Utilities|Array|FindItem (Variables|Default|GetActiveTasks) "Broken Computer") -1)
    (CallFunction|CheckifNeedErrorScreen)
    (else
      (CallFunction|CheckifNeedRemoveErrorScreen))))

(fn CreateErrorScreen
  (bind _errorscreenlocation (Variables|Default|GetErrorScreenLocation))
  (bind _returnvalue (Transformation|GetRelativeTransform _errorscreenlocation))
  (bind _returnvalue_2 (Game|SpawnActorfromClass "/Game/Assets/Props/TaskTablet/BP_Broken_Tablet_Screen.BP_Broken_Tablet_Screen_C" (Transformation|GetActorTransform) "Undefined" "MultiplyWithRoot" 0 0))
  (Transformation|AttachComponentToComponent _returnvalue_2 _errorscreenlocation "None" "KeepRelative" "KeepRelative" "KeepRelative" true)
  (Transformation|SetActorRelativeLocation _returnvalue_2 (.location _returnvalue))
  (Transformation|SetActorRelativeRotation _returnvalue_2 (.rotation _returnvalue)))
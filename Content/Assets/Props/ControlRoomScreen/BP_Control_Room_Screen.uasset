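; Submarine control room screen prop that shows hull health, player money, current and best depth, and ascent or descent arrows.
; Every Tick it polls GS_Core and the first player's CD_PlayerState wallet to rewrite the text, toggling arrows by comparing the submarine state enum as a string.
; It also polls BP_TaskManager, spawning an attached error screen while "Broken Computer" is active and destroying it otherwise, using world-wide class lookups to avoid duplicates.
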(event EventTick
  (params (DeltaSeconds :type Float%20%28single-precision%29))
  (CallFunction|CheckandHandleErrorScreen)
  (CallFunction|UpdateSubmarineHealth)
  (bind _asgs_core (CallFunction|UpdateMoney))
  (bind _asgs_core_2 (CallFunction|UpdateDepth _asgs_core))
  (CallFunction|UpdateBestDepth)
  (CallFunction|UpdateArrow _asgs_core_2))

(fn ConstructionScript)

(fn UpdateMoney
  (bind _ascd_player_state (Utilities|Casting|CastToCD_PlayerState (Game|GetPlayerState 0)))
  (bind _returnvalue (Class|Wallet|GetBalance (Variables|/Script/CrushDepth.CD_PlayerState|Getwallet _ascd_player_state)))
  (Variables|/Script/Text3D.Text3DComponent|SetText (Variables|Default|GetTotalMoneyVar) (Utilities|Text|ToText(String) (Utilities|String|Append "$" (Utilities|String|ToString(Text) (Utilities|Text|ToText(Float) _returnvalue "HalfToEven" false true 1 324 2 2)))))
  (bind _asgs_core (Utilities|Casting|CastToGS_Core (Game|GetGameState))
    (:then
      _)
    (:CastFailed
      _))
  (return _asgs_core))

(fn UpdateDepth
  (params (self2 :type GS%20Core%20Object%20Reference))
  (bind _returnvalue (Class|GSCore|GetSubmarineDepth self2))
  (Variables|/Script/Text3D.Text3DComponent|SetText (Variables|Default|GetCurrentDepthVar) (Utilities|Text|ToText(String) (Utilities|String|Append (Utilities|String|ToString(Text) (Utilities|Text|ToText(String) (Utilities|String|ToString(Integer) (Math|Float|Round _returnvalue)))) "m")))
  (bind _asgs_core (Utilities|Casting|CastToGS_Core (Game|GetGameState)))
  (return _asgs_core))

(fn UpdateArrow
  (params (NewParam :type GS%20Core%20Object%20Reference))
  (bind _returnvalue (Class|GSCore|GetSubmarineState NewParam))
  (if (Utilities|Enum|Equal(Enum) "Descending" (Utilities|String|EnumtoString _returnvalue))
    (Rendering|SetVisibility (Variables|Default|GetDownArrow) true false)
    (elif (Utilities|Enum|Equal(Enum) "Ascending" (Utilities|String|EnumtoString _returnvalue))
      (Rendering|SetVisibility (Variables|Default|GetUpArrowStem) true false)
      (Rendering|SetVisibility (Variables|Default|GetDownArrow) false false)
      (else
        (Rendering|SetVisibility (Variables|Default|GetDownArrow) false false)))))

(fn UpdateSubmarineHealth
  (bind _asgs_core (Utilities|Casting|CastToGS_Core (Game|GetGameState)))
  (bind _returnvalue (Class|GSCore|GetSubmarineHealth _asgs_core))
  (Variables|/Script/Text3D.Text3DComponent|SetText (Variables|Default|GetSubmarineHealthVar) (Utilities|Text|ToText(String) (Utilities|String|Append (Utilities|String|ToString(Text) (Utilities|Text|ToText(Float) _returnvalue "HalfToEven" false true 1 324 2 2)) "%"))))

(fn UpdateBestDepth
  (bind _asgs_core (Utilities|Casting|CastToGS_Core (Game|GetGameState)))
  (bind _returnvalue (Class|GSCore|GetCurrentBestAttempt _asgs_core))
  (Variables|/Script/Text3D.Text3DComponent|SetText (Variables|Default|GetBestDepth) (Utilities|Text|ToText(String) (Utilities|String|Append (Utilities|String|Append "Best: " (Utilities|String|ToString(Text) (Utilities|Text|ToText(Float) _returnvalue "HalfToEven"))) "m"))))

(fn CheckandHandleErrorScreen
  (bind _returnvalue (Actor|GetActorOfClass "/Game/Assets/Tasks/Templates/BP_TaskManager.BP_TaskManager_C"))
  (bind _tasknames (Default|GetActiveTasks _returnvalue))
  (if (Utilities|Array|ContainsItem _tasknames "Broken Computer")
    (CallFunction|CheckifComputerError)
    (else
      (CallFunction|RemoveErrorScreen))))

(fn CreateandAttachErrorScreen
  (bind _errorscreenlocation (Variables|Default|GetErrorScreenLocation))
  (bind _returnvalue (Transformation|GetRelativeTransform _errorscreenlocation))
  (bind _returnvalue_2 (Game|SpawnActorfromClass "/Game/Assets/Props/ControlRoomScreen/BP_Control_Room_Error_Screen.BP_Control_Room_Error_Screen_C" (Transformation|GetActorTransform) "Undefined" "MultiplyWithRoot" 0 0))
  (Transformation|AttachComponentToComponent _returnvalue_2 _errorscreenlocation "None" "KeepRelative" "KeepRelative" "KeepRelative" true)
  (Transformation|SetActorRelativeLocation _returnvalue_2 (.location _returnvalue))
  (Transformation|SetActorRelativeRotation _returnvalue_2 (.rotation _returnvalue)))

(fn RemoveErrorScreen
  (bind _returnvalue (Actor|GetActorOfClass "/Game/Assets/Props/ControlRoomScreen/BP_Control_Room_Error_Screen.BP_Control_Room_Error_Screen_C"))
  (if (Utilities|IsValid _returnvalue)
    (Actor|DestroyActor _returnvalue)))

(fn CheckifComputerError
  (bind _outactors (Actor|GetAllActorsOfClass "/Game/Assets/Props/ControlRoomScreen/BP_Control_Room_Error_Screen.BP_Control_Room_Error_Screen_C"))
  (if (Utilities|Array|IsEmpty _outactors)
    (CallFunction|CreateandAttachErrorScreen)))
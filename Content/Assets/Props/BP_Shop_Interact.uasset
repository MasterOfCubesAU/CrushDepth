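; Interactable shop prop that opens the shop widget for the first player when the submarine is surfaced.
; Interaction checks the submarine state from GS_Core by comparing its enum name to "Surfaced".
; Regardless of that result, it locks move and look input, shows the cursor, blends the view to itself and sets the player state to InTask.
; IgnoreInputs is empty, and NewFunction, holding the not-surfaced debug message, is never called here.
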(event EventInteraction
  (bind _returnvalue (Game|GetPlayerController 0))
  (bind _returnvalue_2 (CallFunction|CheckifSurfaced))
  (if _returnvalue_2
    (bind _returnvalue_3 (UserInterface|CreateWidget "/Game/UI/WB_ShopWidget.WB_ShopWidget_C" _returnvalue))
    (UserInterface|Viewport|AddtoViewport _returnvalue_3 0))
  (Input|SetIgnoreMoveInput _returnvalue true)
  (Input|SetIgnoreLookInput _returnvalue true)
  (CallFunction|IgnoreInputs)
  (Variables|/Script/Engine.PlayerController|SetbShowMouseCursor _returnvalue true)
  (Game|Player|SetViewTargetwithBlend _returnvalue self 0.0 "VTBlend_Linear" 0.0 false)
  (bind _ascd_player_state (Utilities|Casting|CastToCD_PlayerState (Game|GetPlayerState 0))
    (:then
      _)
    (:CastFailed
      _))
  (Class|CDPlayerState|SetPlayerState _ascd_player_state "InTask"))

(fn ConstructionScript)

(fn IgnoreInputs)

(fn NewFunction
  (bind _asgs_core (Utilities|Casting|CastToGS_Core (Game|GetGameState))
    (:then
      _)
    (:CastFailed
      _))
  (bind _returnvalue (Class|GSCore|GetSubmarineState _asgs_core))
  (if (Utilities|Enum|Equal(Enum) (Utilities|String|EnumtoString _returnvalue) "Surfaced")
    _
    (else
      (Development|PrintString "Cannot access shop whilst not surfaced")))
  (return (Game|GetPlayerController 0)))

(fn CheckifSurfaced
  (bind _asgs_core (Utilities|Casting|CastToGS_Core (Game|GetGameState))
    (:then
      _)
    (:CastFailed
      _))
  (bind _returnvalue (Class|GSCore|GetSubmarineState _asgs_core))
  (return (Utilities|Enum|Equal(Enum) (Utilities|String|EnumtoString _returnvalue) "Surfaced")))
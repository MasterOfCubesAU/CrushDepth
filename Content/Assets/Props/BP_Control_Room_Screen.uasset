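; Control room screen prop that shows the player's money, submarine depth, travel direction, best depth and hull health.
; Every Tick it polls the first player's wallet and the GS_Core game state, with the money and depth updates handing the game state along.
; Direction arrows follow the submarine state by enum name, though descending never hides the up arrow.
; Best depth refreshes only while neither ascending nor descending.
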(event EventTick
  (params (DeltaSeconds :type Float%20%28single-precision%29))
  (bind _asgs_core (CallFunction|UpdateMoney))
  (bind _asgs_core_2 (CallFunction|UpdateDepth _asgs_core))
  (CallFunction|UpdateArrow _asgs_core_2)
  (CallFunction|UpdateSubmarineHealth))

(fn ConstructionScript)

(fn UpdateMoney
  (bind _ascd_player_state (Utilities|Casting|CastToCD_PlayerState (Game|GetPlayerState 0)))
  (bind _returnvalue (Class|Wallet|GetBalance (Variables|/Script/CrushDepth.CD_PlayerState|Getwallet _ascd_player_state)))
  (Variables|/Script/Text3D.Text3DComponent|SetText (Variables|Default|GetTotalMoneyVar) (Utilities|Text|ToText(String) (Utilities|String|Append "$" (Utilities|String|ToString(Text) (Utilities|Text|ToText(Float) _returnvalue "HalfToEven" false true 1 324 2 2)))))
  (bind _asgs_core (Utilities|Casting|CastToGS_Core (Game|GetGameState))
    (:then
      _)
    (:CastFailed
      _))
  (return _asgs_core))

(fn UpdateDepth
  (params (self2 :type GS%20Core%20Object%20Reference))
  (bind _returnvalue (Class|GSCore|GetSubmarineDepth self2))
  (Variables|/Script/Text3D.Text3DComponent|SetText (Variables|Default|GetCurrentDepthVar) (Utilities|Text|ToText(String) (Utilities|String|Append (Utilities|String|ToString(Text) (Utilities|Text|ToText(String) (Utilities|String|ToString(Integer) (Math|Float|Round _returnvalue)))) "m")))
  (bind _asgs_core (Utilities|Casting|CastToGS_Core (Game|GetGameState)))
  (return _asgs_core))

(fn UpdateArrow
  (params (NewParam :type GS%20Core%20Object%20Reference))
  (bind _returnvalue (Class|GSCore|GetSubmarineState NewParam))
  (if (Utilities|Enum|Equal(Enum) "Descending" (Utilities|String|EnumtoString _returnvalue))
    (Rendering|SetVisibility (Variables|Default|GetDownArrow) true false)
    (elif (Utilities|Enum|Equal(Enum) "Ascending" (Utilities|String|EnumtoString _returnvalue))
      (Rendering|SetVisibility (Variables|Default|GetUpArrowStem) true false)
      (Rendering|SetVisibility (Variables|Default|GetDownArrow) false false)
      (else
        (Rendering|SetVisibility (Variables|Default|GetDownArrow) false false)
        (bind _asgs_core (Utilities|Casting|CastToGS_Core (Game|GetGameState)))
        (bind _returnvalue_2 (Class|GSCore|GetCurrentBestAttempt _asgs_core))
        (Variables|/Script/Text3D.Text3DComponent|SetText (Variables|Default|GetBestDepth) (Utilities|Text|ToText(String) (Utilities|String|Append (Utilities|String|Append "Best: " (Utilities|String|ToString(Text) (Utilities|Text|ToText(Float) _returnvalue_2 "HalfToEven"))) "m")))))))

(fn UpdateSubmarineHealth
  (bind _asgs_core (Utilities|Casting|CastToGS_Core (Game|GetGameState)))
  (bind _returnvalue (Class|GSCore|GetSubmarineHealth _asgs_core))
  (Variables|/Script/Text3D.Text3DComponent|SetText (Variables|Default|GetSubmarineHealthVar) (Utilities|Text|ToText(String) (Utilities|String|Append (Utilities|String|ToString(Text) (Utilities|Text|ToText(Float) _returnvalue "HalfToEven" false true 1 324 2 2)) "%"))))
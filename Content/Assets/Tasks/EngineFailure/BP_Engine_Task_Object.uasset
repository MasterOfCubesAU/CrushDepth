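; Engine Failure task actor, a repair puzzle where missing gears must be replaced.
; Setup swaps a random subset of replaced-gear actors for missing-gear actors, counts them and turns the indicator lights to warning.
; It polls GearsLeft every 0.2 seconds, then restores green lights and solves the task at zero.
; Interaction blends the view to this actor, shows the cursor, ignores move/look input and sets the player state to InTask.
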(event EventBeginPlay
  (Variables|Default|SetName "Engine Failure"))

(event EventSetupTask
  ;[1 1 1] Setup the task and run in a loop to detect whether task if finished
  (CallFunction|StartTask)
  (Utilities|FlowControl|Delay 0.2 :!label _label)
  (if (<= (Variables|Default|GetGearsLeft) 0)
    (CallFunction|FinishTask)
    (CallFunction|SolveTask)
    (else
      (goto _label))))

(event EventInteraction
  ;[1 1 1] Handle Player Interacting with Task - Switch camera to focus on task
  (CallFunction|FocusonTask))

(fn ConstructionScript)

(fn StartTask
  ;[1 1 1] Start task - set missing gears, calculate number of missing gears and set task appearance
  (CallFunction|SetMissingGears)
  (CallFunction|SetGearNumbers)
  (CallFunction|SetTaskAppearance true))

(fn FinishTask
  ;[1 1 1] Change appearance to green light again
  (CallFunction|SetTaskAppearance false))

(fn IgnoreInputs
  (bind _returnvalue (Game|GetPlayerController 0))
  (Variables|/Script/Engine.PlayerController|SetbShowMouseCursor _returnvalue true)
  (Input|SetIgnoreMoveInput _returnvalue true)
  (Input|SetIgnoreLookInput _returnvalue true))

(fn EnableInputs
  (bind _returnvalue (Game|GetPlayerController 0))
  (if (and (Class|Controller|IsMoveInputIgnored _returnvalue) (Class|Controller|IsLookInputIgnored _returnvalue))
    (Input|ResetIgnoreMoveInput _returnvalue)
    (Input|ResetIgnoreLookInput _returnvalue)))

(fn SetGearNumbers
  (bind _outactors (Actor|GetAllActorsOfClass "/Game/Assets/Tasks/EngineFailure/BP_Missing_Gear.BP_Missing_Gear_C"))
  (bind _output_get (Variables|Default|SetGearsLeft (Utilities|Array|Length _outactors)))
  (Variables|Default|SetTotalMissingGears _output_get))

(fn SetTaskAppearance
  (params (IsTaskActive :type Boolean))
  ;[1 1 1] Set lights based on whether task is active
  (if IsTaskActive
    (Rendering|Material|SetMaterial (Variables|Default|GetIndicatorLight) 0 "/Game/Assets/Material/M_Warning_Light.M_Warning_Light")
    (Rendering|Components|Light|SetLightColor (Variables|Default|GetPointLight) (Variables|Default|GetError%20colour) true)
    (else
      (Rendering|Material|SetMaterial (Variables|Default|GetIndicatorLight) 0 "/Game/Assets/Material/M_Green_Light.M_Green_Light")
      (Rendering|Components|Light|SetLightColor (Variables|Default|GetPointLight) (Variables|Default|GetSuccess%20colour) true))))

(fn SetMissingGears
  ;[1 1 1] Set the missing gears that need to be replaced to fix the task
  (bind _outactors (Actor|GetAllActorsOfClass "/Game/Assets/Tasks/EngineFailure/BP_Replaced_Gear.BP_Replaced_Gear_C"))
  (bind _output_get (LocalVariables|SetgearArray _outactors))
  (Utilities|Array|Shuffle _output_get)
  (LocalVariables|SetnumGears (Math|Random|RandomIntegerinRange 1 (- (Utilities|Array|Length _outactors) 1)))
  (while (> (LocalVariables|GetnumGears) 0) :!label _label
    (Game|SpawnActorfromClass "/Game/Assets/Tasks/EngineFailure/BP_Missing_Gear.BP_Missing_Gear_C" (Transformation|GetActorTransform (Utilities|Array|Get(acopy) (LocalVariables|GetgearArray) (LocalVariables|GetnumGears))) "Undefined" "MultiplyWithRoot" 0 0)
    (Actor|DestroyActor (Utilities|Array|Get(acopy) (LocalVariables|GetgearArray) (LocalVariables|GetnumGears)))
    (bind _result (Math|Integer|DecrementInt (LocalVariables|GetnumGears))
      (:%20%20
        (LocalVariables|SetnumGears _result)
        (goto _label)))))

(fn FocusonTask
  ;[1 1 1] Switch camera to the task camera and disable look and movement inputs
  (CallFunction|IgnoreInputs)
  (Game|Player|SetViewTargetwithBlend (Game|GetPlayerController 0) self 0.0 "VTBlend_Linear" 0.0 false)
  (bind _ascd_player_state (Utilities|Casting|CastToCD_PlayerState (Game|GetPlayerState 0)))
  (Class|CDPlayerState|SetPlayerState _ascd_player_state "InTask"))
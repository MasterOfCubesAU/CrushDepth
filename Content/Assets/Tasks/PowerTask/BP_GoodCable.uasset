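; BP_GoodCable is a clickable cable in the power task that triggers a timed reaction when clicked.
; ProcessClick teleport-free moves the BP_Power actor's Block to a fixed position and shows the WrongText actor's Wrong component, despite the cable's "good" name.
; A two-second function-name timer calls VerifyGoBack, whose GoBack call hides the text and moves the Block back.
; Both target actors are found by class lookup, and the verify event is empty.
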(event Custom|verify)

(event EventProcessClick
  ;[1 1 1] Setting 2 second delay after click on good cable
  (bind _returnvalue (Actor|GetActorOfClass "/Game/Assets/Tasks/PowerTask/BP_Power.BP_Power_C"))
  (Transformation|SetWorldLocation (Variables|/Game/Assets/Tasks/PowerTask/BP_Power.BP_Power_C|Getblock _returnvalue) "-140.000000,640.000000,140.000000" false false)
  (bind _returnvalue_2 (Actor|GetActorOfClass "/Game/Assets/Tasks/PowerTask/WrongText.WrongText_C"))
  (Rendering|SetVisibility (Variables|/Game/Assets/Tasks/PowerTask/WrongText.WrongText_C|GetWrong _returnvalue_2) true false)
  (Utilities|Time|SetTimerbyFunctionName 0 "VerifyGoBack" 2.0))

(fn ConstructionScript)

(fn GoBack
  (bind _returnvalue (Actor|GetActorOfClass "/Game/Assets/Tasks/PowerTask/WrongText.WrongText_C"))
  (Rendering|SetVisibility (Variables|/Game/Assets/Tasks/PowerTask/WrongText.WrongText_C|GetWrong _returnvalue) false false)
  (bind _returnvalue_2 (Actor|GetActorOfClass "/Game/Assets/Tasks/PowerTask/BP_Power.BP_Power_C"))
  (Transformation|SetWorldLocation (Variables|/Game/Assets/Tasks/PowerTask/BP_Power.BP_Power_C|Getblock _returnvalue_2) "-300.000000,640.000000,140.000000" false false))

(fn VerifyGoBack
  (CallFunction|GoBack))
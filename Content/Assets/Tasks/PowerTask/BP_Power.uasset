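; BP_Power is a task actor for a power task, solved when the player pawn overlaps it.
; The SetupTask event teleports the Cube component to a raised relative position.
; The player's overlap lowers the Cube back to its relative origin and calls SolveTask.
; Author comments mark the setup as a TODO and the overlap logic as a changeable example, so the behavior appears to be placeholder.
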(event EventBeginPlay)

(event EventSetupTask
  ;[1 1 1] TODO: Implement this - Setup for the stuff in Components (left side, viewport stuff) Change as you like, as long as comes from the EventSetupTask node
  (Transformation|SetRelativeLocation (Variables|Default|GetCube) "0.000000,0.000000,50.000000" false true))

(event EventTick
  (params (DeltaSeconds :type Float%20%28single-precision%29)))

(event Collision|EventActorBeginOverlap
  (params (OtherActor :type Actor%20Object%20Reference))
  ;[1 1 1] Example of above, change this as you like, be sure to have a call to SolveTask
  (if (== OtherActor (Game|Player|GetPlayerPawn 0))
    (Transformation|SetRelativeLocation (Variables|Default|GetCube) "0, 0, 0" false false)
    (CallFunction|SolveTask)))

(fn ConstructionScript
  (|CallParentFunction))
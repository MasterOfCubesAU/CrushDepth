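; Miscalibration task where the player reboots broken screens by dragging a lever with the mouse in a focused task view.
; Setup shows a reboot warning and randomly breaks screens; the lever follows the cursor through a delay loop, clamped vertically between two hitboxes.
; Hitting the reboot hitbox springs the lever back via timeline and starts a countdown.
; A further pull after it ends fixes the screens and solves the task.
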(event OnComponentBeginOverlap(RebootHitbox)
  (params (OverlappedComponent :type Primitive%20Component%20Object%20Reference) (OtherActor :type Actor%20Object%20Reference) (OtherComp :type Primitive%20Component%20Object%20Reference) (OtherBodyIndex :type Integer) (bFromSweep :type Boolean) (SweepResult :type Hit%20Result%20Structure%20%28by%20ref%29))
  (bind _returnvalue (Utilities|Time|GetGameTimeinSeconds))
  (if (and (Variables|Default|GetIsActive) (== OtherComp (Variables|Default|GetleverHitbox)))
    (Variables|Default|SetIsHeld false)
    (Utilities|FlowControl|Delay 0.1)
    (CallFunction|EventRestartLever)
    (if (== (Variables|Default|GetTimer) 0.0)
      (Variables|Default|SetTimer _returnvalue)
      ;[1 1 1] Pity system
      (Variables|Default|SetActivateTime _returnvalue)
      (bind _returnvalue_2 (CallFunction|GetRemainingTimer :!label _label))
      (if (== _returnvalue_2 0)
        (CallFunction|SetRebootString)
        (Rendering|Material|SetMaterial (Variables|Default|GetStatusScreen) 0 "/Game/Assets/Material/M_Green_Light.M_Green_Light")
        (Variables|Default|SetRebootSuccess true)
        (else
          (CallFunction|SetRebootString _returnvalue_2)
          (Utilities|FlowControl|Delay 1.0)
          (goto _label)))
      (else
        (CallFunction|EventCheckSuccess)))))

(event Custom|Event%20Check%20success
  (if (Variables|Default|GetRebootSuccess)
    (CallFunction|FixWarningScreen)
    (Rendering|Material|SetMaterial (Variables|Default|GetStatusScreen) 0 "/Game/Assets/Material/M_Screen_Light.M_Screen_Light")
    (CallFunction|FixScreens)
    (CallFunction|SolveTask)))

(event Custom|Event%20Restart%20Lever
  (bind _levercore (Variables|Default|GetLeverCore))
  (bind _returnvalue (Transformation|GetWorldLocation _levercore))
  (Variables|Default|SetOldLocation _returnvalue)
  (bind _lerp (Timeline|Reset%20lever Play)
    (:Update
      (Transformation|SetWorldLocation (Variables|Default|GetLeverCore) (Math|Vector|Lerp(Vector) _returnvalue (Transformation|GetWorldLocation (Variables|Default|GetLeverStart)) _lerp) false false))))

(event EventBeginPlay
  (Variables|Default|SetName "Miscalibration")
  (bind _asbp_first_person_player_controller (Utilities|Casting|CastToBP_FirstPersonPlayerController (Game|GetPlayerController 0)))
  (Variables|Default|SetPlayer%20Controller _asbp_first_person_player_controller)
  (CallFunction|MakeScreenArray)
  (Rendering|SetVisibility (Variables|Default|GetleverHitbox) false false))

(event EventSetupTask
  (Variables|Default|SetTimer 0.0)
  (Variables|Default|SetRebootSuccess false)
  (CallFunction|SetWarningScreen)
  (CallFunction|BreakScreens)
  (CallFunction|ResetLeverLocation))

(event EventInteraction
  (CallFunction|FocusonTask))

(event EventProcessClick
  (if (Class|Controller|IsMoveInputIgnored (Game|GetPlayerController 0))
    (Variables|Default|SetIsHeld true)
    (bind _cursorlocation (CallFunction|CursorLocation))
    (if (<= (Math|Vector|Distance(Vector) _cursorlocation (Transformation|GetWorldLocation (Variables|Default|GetleverHitbox))) 1e+01)
      (if (Variables|Default|GetIsHeld) :!label _label
        (bind _cursorlocation_2 (CallFunction|CursorLocation))
        (Transformation|SetWorldLocation (Variables|Default|GetLeverCore) _cursorlocation_2 false false)
        (Utilities|FlowControl|Delay 0.01)
        (goto _label)))))

(event EventReleaseClick
  (Variables|Default|SetIsHeld false)
  (Utilities|FlowControl|Delay 0.1)
  (CallFunction|EventRestartLever)
  (Transformation|SetWorldLocation (Variables|Default|GetLeverCore) (Transformation|GetWorldLocation (Variables|Default|GetLeverStart)) false false))

(fn ConstructionScript
  (|CallParentFunction))

(fn IgnoreInputs
  (bind _returnvalue (Game|GetPlayerController 0))
  (Variables|/Script/Engine.PlayerController|SetbShowMouseCursor _returnvalue true)
  (Input|SetIgnoreMoveInput _returnvalue true)
  (Input|SetIgnoreLookInput _returnvalue true))

(fn FocusonTask
  (CallFunction|IgnoreInputs)
  (Game|Player|SetViewTargetwithBlend (Game|GetPlayerController 0) self 0.0 "VTBlend_Linear" 0.0 false)
  (bind _ascd_player_state (Utilities|Casting|CastToCD_PlayerState (Game|GetPlayerState 0)))
  (Class|CDPlayerState|SetPlayerState _ascd_player_state "InTask"))

(fn CursorLocation
  (bind _leverhitbox (Variables|Default|GetleverHitbox))
  (bind _returnvalue (Transformation|GetWorldLocation _leverhitbox))
  (return (Math|Vector|MakeVector (.x _returnvalue) (.y _returnvalue) (Math|Float|Clamp(Float) (.z (.Location (Collision|BreakHitResult (.HitResult (Game|Player|GetHitResultUnderCursorbyChannel (Variables|Default|GetPlayer%20Controller) "TraceTypeQuery1" false))))) (.z (Transformation|GetWorldLocation (Variables|Default|GetRebootHitbox))) (.z _returnvalue)))))

(fn BreakScreens
  (for _array_element (Variables|Default|GetScreens)
    (if (Math|Random|RandomBool)
      (Rendering|Material|SetMaterial _array_element 0 "/Game/Assets/Material/M_Warning_Light.M_Warning_Light"))))

(fn FixScreens
  (for _array_element (Variables|Default|GetScreens)
    (Rendering|Material|SetMaterial _array_element 0 "/Game/Assets/Material/M_Screen_Light.M_Screen_Light")))

(fn ResetLeverLocation
  (Transformation|SetRelativeLocation (Variables|Default|GetLeverCore) (Variables|/Script/Engine.SceneComponent|GetRelativeLocation (Variables|Default|GetLeverStart)) false true))

(fn MakeScreenArray
  (bind _screens (Variables|Default|GetScreens))
  (Utilities|Array|AppendArray _screens (Utilities|Array|MakeArray (Variables|Default|GetPlane1)))
  (Utilities|Array|AppendArray _screens (Utilities|Array|MakeArray (Variables|Default|GetStaticMesh)))
  (Utilities|Array|AppendArray _screens (Utilities|Array|MakeArray (Variables|Default|GetStaticMesh1)))
  (Utilities|Array|AppendArray _screens (Utilities|Array|MakeArray (Variables|Default|GetStaticMesh2)))
  (Utilities|Array|AppendArray _screens (Utilities|Array|MakeArray (Variables|Default|GetStaticMesh3)))
  (Utilities|Array|AppendArray _screens (Utilities|Array|MakeArray (Variables|Default|GetStaticMesh4)))
  (Utilities|Array|AppendArray _screens (Utilities|Array|MakeArray (Variables|Default|GetStaticMesh5))))

(fn GetRemainingTimer
  (return (Math|Integer|Clamp(Integer) (Math|Float|Truncate (- (Variables|Default|GetTimerLength) (- (Utilities|Time|GetGameTimeinSeconds) (Variables|Default|GetTimer)))) 0 60)))

(fn SetRebootString
  (params (InInt :type Integer))
  (Rendering|Components|TextRender|SetText (Variables|Default|GetTextRender1) (Utilities|Text|ToText(String) (Utilities|String|BuildString(Integer) "Reboot in " "" InInt))))

(fn SetWarningScreen
  (Rendering|Components|TextRender|SetText (Variables|Default|GetTextRender1) (Utilities|Text|ToText(String) "Reboot Required"))
  (Rendering|Material|SetMaterial (Variables|Default|GetStatusScreen) 0 "/Game/Assets/Material/M_Warning_Light.M_Warning_Light"))

(fn FixWarningScreen
  (Rendering|Components|TextRender|SetText (Variables|Default|GetTextRender1) (Utilities|Text|ToText(String) "Status Normal")))
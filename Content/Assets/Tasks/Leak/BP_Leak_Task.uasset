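; Leak task that, on setup, plays a leak announcement through the PA system and spawns two leaks in the level.
; Spawn transforms come from the BP_Leak_Location markers placed in the level, shuffled so that each setup picks two at random.
; LeakCheck, meant to run whenever a leak is solved, counts the remaining BP_Leak actors and solves the task when none are left.
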(event Custom|LeakCheck
  ;[1 1 1] For every leak that is solved, check that the total count is zero
  (bind _outactors (Actor|GetAllActorsOfClass "/Game/Assets/Tasks/Leak/BP_Leak.BP_Leak_C"))
  (if (== (Utilities|Array|Length _outactors) 0)
    (CallFunction|SolveTask)))

(event EventBeginPlay
  (Variables|Default|SetName "Leak Task"))

(event EventSetupTask
  ;[1 1 1] Play announcement sound
  (bind _returnvalue (Actor|GetActorOfClass "/Script/CrushDepth.PA_System"))
  (Class|PASystem|PlayAnnouncement _returnvalue "leak_detected")
  ;[1 1 1] Spawn leaks
  (CallFunction|SpawnLeaks))

(fn ConstructionScript)

(fn SpawnLeaks
  ;[1 1 1] Randomise the list of leak locations and pick 2
  (CallFunction|GetLeakLocations)
  (CallFunction|GenerateLeaksinLevel))

(fn GetLeakLocations
  ;[1 1 1] Look for leak spawn objects in level and create a list
  (bind _outactors (Actor|GetAllActorsOfClass "/Game/Assets/Tasks/Leak/BP_Leak_Location.BP_Leak_Location_C"))
  (for _array_element _outactors
    (Utilities|Array|Add (Variables|Default|GetLeakSpawns) (Transformation|GetActorTransform _array_element)))
  (bind _output_get (Variables|Default|SetRandomisedSpawns (Variables|Default|GetLeakSpawns)))
  (Utilities|Array|Shuffle _output_get))

(fn GenerateLeaksinLevel
  ;[1 1 1] Randomise list of spawns and pick 2 locations
  (for _index (range 0 1)
    (Game|SpawnActorfromClass "/Game/Assets/Tasks/Leak/BP_Leak.BP_Leak_C" (Math|Transform|MakeTransform (Math|Transform|TransformLocation (Utilities|Array|Get(acopy) (Variables|Default|GetRandomisedSpawns) _index) "0, 0, 0") (Math|Transform|TransformRotation (Utilities|Array|Get(acopy) (Variables|Default|GetRandomisedSpawns) _index) "0, 0, 0") "1.000000,1.000000,1.000000") "Undefined" "MultiplyWithRoot" 0 0)))
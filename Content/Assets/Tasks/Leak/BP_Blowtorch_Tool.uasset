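; Blowtorch tool for the leak task that the player picks up, holds to use, and drops.
; While use is held, a 0.01-second delay loop keeps spawned sparks at the nozzle along the player's aim and flicks RepairParticle between nozzle and world origin.
; Release destroys the sparks.
; Pickup disables collision; dropping restores it with physics, then five seconds later calls respawn if IsPlayerHoldingThis returns true.
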(event EventDropItem
  (bind _physicsroot (Variables|Default|GetPhysicsRoot))
  (CallFunction|EnableCollision (Variables|Default|Getpaint_can_upload))
  (CallFunction|EnableCollision _physicsroot)
  (Physics|SetSimulatePhysics _physicsroot true)
  (Utilities|FlowControl|Delay 5.0)
  (bind _returnvalue (CallFunction|IsPlayerHoldingThis))
  (if _returnvalue
    (CallFunction|HandleItemRespawn)))

(event EventInteraction
  (CallFunction|HandlePickup)
  (CallFunction|DisableCollision (Variables|Default|GetPhysicsRoot))
  (CallFunction|DisableCollision (Variables|Default|Getpaint_can_upload)))

(event EventProcessUse
  (bind _repairparticle (Variables|Default|GetRepairParticle))
  (bind _emitter (Variables|Default|Getemitter))
  (bind _returnvalue (Transformation|GetWorldLocation _emitter))
  (bind _returnvalue_2 (Transformation|GetWorldRotation _emitter))
  (bind _returnvalue_3 (+ _returnvalue _returnvalue_2))
  (Variables|Default|SetHeldDown true)
  (bind _returnvalue_4 (Effects|SpawnEmitteratLocation "/Game/StarterContent/Particles/P_Sparks.P_Sparks" _returnvalue_3))
  (if (Variables|Default|GetHeldDown) :!label _label
    (Transformation|SetWorldLocationAndRotation _returnvalue_4 _returnvalue_3 (Pawn|GetBaseAimRotation (Game|Player|GetPlayerPawn 0)) false false)
    (Transformation|SetWorldLocation _repairparticle _returnvalue_3 false false)
    (Utilities|FlowControl|Delay 0.01)
    (Transformation|SetWorldLocation _repairparticle "0, 0, 0" false false)
    (goto _label)
    (else
      (Transformation|SetWorldLocation _repairparticle "0, 0, 0" false false))))

(event EventReleaseUse
  (Variables|Default|SetHeldDown false)
  (Components|DestroyComponent (stale EventProcessUse _returnvalue_4)))

(fn ConstructionScript)
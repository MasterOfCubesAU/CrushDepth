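; BP_Fire is an extinguishable fire actor that spawns a P_Fire particle effect at its location on BeginPlay.
; Each Box overlap by a component named "FireExtParticles" lowers its Integrity by one and prints the new value.
; When Integrity runs out, it destroys itself and the effect, then calls FireCheck on the BP_Fire_Task actor found in the level.
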(event OnComponentBeginOverlap(Box)
  (params (OverlappedComponent :type Primitive%20Component%20Object%20Reference) (OtherActor :type Actor%20Object%20Reference) (OtherComp :type Primitive%20Component%20Object%20Reference) (OtherBodyIndex :type Integer) (bFromSweep :type Boolean) (SweepResult :type Hit%20Result%20Structure%20%28by%20ref%29))
  (bind _integrity (Variables|Default|GetIntegrity))
  (if (Utilities|Enum|Equal(Enum) (Utilities|GetObjectName OtherComp) "FireExtParticles")
    (Math|Integer|DecrementInt _integrity
      (:%20%20
        (Development|PrintString (Utilities|String|BuildString(Integer) "Integrity dropped to " "" _integrity))
        (if (<= _integrity 0)
          (Actor|DestroyActor)
          (Components|DestroyComponent (stale EventBeginPlay _returnvalue))
          (bind _returnvalue (Actor|GetActorOfClass "/Game/Assets/Tasks/Fire/BP_Fire_Task.BP_Fire_Task_C"))
          (Default|FireCheck _returnvalue))))))

(event EventBeginPlay
  (bind _returnvalue (Effects|SpawnEmitteratLocation "/Game/StarterContent/Particles/P_Fire.P_Fire" (Transformation|GetActorLocation self))))

(event Collision|EventActorBeginOverlap
  (params (OtherActor :type Actor%20Object%20Reference)))

(event EventTick
  (params (DeltaSeconds :type Float%20%28single-precision%29)))

(fn ConstructionScript)
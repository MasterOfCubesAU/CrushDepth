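; Task Blueprint for a "Fire Outbreak" event, in which fires break out at either the engine or power spawn points.
; On setup it picks one of the two location arrays at random and spawns a BP_Fire at each entry.
; FireCheck solves the task when no BP_Fire actors remain in the world, and also runs right after spawning as a fallback for failed spawns.
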(event Custom|FireCheck
  (bind _outactors (Actor|GetAllActorsOfClass "/Game/Assets/Tasks/Fire/BP_Fire.BP_Fire_C"))
  (if (== (Utilities|Array|Length _outactors) 0)
    (CallFunction|SolveTask)))

(event EventBeginPlay
  (Variables|Default|SetName "Fire Outbreak")
  (Input|EnableInput (Game|GetPlayerController 0)))

(event EventSetupTask
  (if (Math|Random|RandomBool)
    (CallFunction|SpawnFires (Variables|Default|GetEngineSpawns))
    (else
      (CallFunction|SpawnFires (Variables|Default|GetPowerSpawns))))
  ;[1 1 1] In case failure of spawn
  (CallFunction|FireCheck))

(event EventTick
  (params (DeltaSeconds :type Float%20%28single-precision%29)))

(event Input|KeyboardEvents|B
  (params (Key :type Key%20Structure :default "None")))

(fn ConstructionScript
  (|CallParentFunction))

(fn SpawnFires
  (params (Array :type Array%20of%20Vectors))
  (for _array_element Array
    (Game|SpawnActorfromClass "/Game/Assets/Tasks/Fire/BP_Fire.BP_Fire_C" (Math|Transform|MakeTransform _array_element "0, 0, 0" "1.000000,1.000000,1.000000") "Undefined" "MultiplyWithRoot" 0 0)))
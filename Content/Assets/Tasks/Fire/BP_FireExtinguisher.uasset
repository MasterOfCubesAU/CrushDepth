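; BP_FireExtinguisher is a fire extinguisher that sprays while its use action is held.
; ProcessUse spawns the spray emitter at FireSpawn, then a 0.01-second Delay loop keeps it aligned with that point until ReleaseUse clears HeldDown and destroys it.
; Each loop also pulses FireExtParticles between the Hitbox location and the world origin, parking it at the origin when spraying stops.
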(event Collision|EventActorBeginOverlap
  (params (OtherActor :type Actor%20Object%20Reference)))

(event EventTick
  (params (DeltaSeconds :type Float%20%28single-precision%29)))

(event EventProcessUse
  (bind _firespawn (Variables|Default|GetFireSpawn))
  (bind _fireextparticles (Variables|Default|GetFireExtParticles))
  (bind _returnvalue (Transformation|GetWorldLocation _firespawn))
  (bind _returnvalue_2 (Transformation|GetWorldRotation _firespawn))
  (Variables|Default|SetHeldDown true)
  (bind _returnvalue_3 (Effects|SpawnEmitteratLocation "/Game/Assets/Tasks/Fire/P_FireExt.P_FireExt" _returnvalue _returnvalue_2))
  (if (Variables|Default|GetHeldDown) :!label _label
    (Transformation|SetWorldLocationAndRotation _returnvalue_3 _returnvalue _returnvalue_2 false false)
    (Transformation|SetWorldLocation _fireextparticles (Transformation|GetWorldLocation (Variables|Default|GetHitbox)) false false)
    (Utilities|FlowControl|Delay 0.01)
    (Transformation|SetWorldLocation _fireextparticles "0, 0, 0" false false)
    (goto _label)
    (else
      (Transformation|SetWorldLocation _fireextparticles "0, 0, 0" false false))))

(event EventReleaseUse
  (Variables|Default|SetHeldDown false)
  (Components|DestroyComponent (stale EventProcessUse _returnvalue_3)))

(fn ConstructionScript)
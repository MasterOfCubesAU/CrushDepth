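; BP_Computer is a computer malfunction task that the player solves by clicking the computer.
; SetupTask enables click events, saves the normal screen text, shows a warning and starts a looping one-second timer.
; ProcessClick plays the Hit component and counts clicks.
; The ComputerWin timer restores the text and calls SolveTask once three clicks register within fifteen seconds; it never clears itself or handles a timeout.
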(event EventProcessClick
  (Audio|Components|Audio|Play (Variables|Default|Gethit) 0.0)
  (Variables|Default|SetTimes (+ (Variables|Default|GetTimes) 1)))

(event EventSetupTask
  (Variables|/Script/Engine.PlayerController|SetbEnableClickEvents (Game|GetPlayerController 0) true)
  (Variables|Default|SetNormal (Variables|/Script/Engine.TextRenderComponent|GetText (Variables|Default|GetTextRender)))
  (bind _output_get (Variables|Default|SetWarning "Warning!!"))
  (Rendering|Components|TextRender|SetText (Variables|Default|GetTextRender) _output_get)
  (Utilities|Time|SetTimerbyFunctionName 0 "ComputerWin" 1.0 true))

(fn ConstructionScript
  (|CallParentFunction))

(fn ComputerWin
  (Variables|Default|SetTime (+ (Variables|Default|GetTime) 1.0))
  (if (<= (Variables|Default|GetTime) 15.0)
    (if (>= (Variables|Default|GetTimes) 3)
      (Rendering|Components|TextRender|SetText (Variables|Default|GetTextRender) (Variables|Default|GetNormal))
      (CallFunction|SolveTask))))
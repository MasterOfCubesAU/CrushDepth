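; BP_TaskTemplate is a base template for activatable tasks that deal damage through BP_TaskManager until they are solved.
; EventActivate ignores repeat calls while active, stores the given time, calls the empty SetupTask hook for visual changes, then starts a delay loop.
; Each pass looks up the manager, passes the stored time to DoDamage and waits its DamageDelay.
; SolveTask clears the active flag and prints a debug message.
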(event Custom|EventActivate
  (params (Time :type Float%20%28double-precision%29))
  (if (not (Variables|Default|GetIsActive))
    (Variables|Default|SetActivateTime Time)
    (Variables|Default|SetIsActive true)
    ;[1 1 1] Event Call for changing Viewport stuff of task to become a task
    (CallFunction|SetupTask)
    (if (Variables|Default|GetIsActive) :!label _label
      (bind _returnvalue (Actor|GetActorOfClass "/Game/Assets/Tasks/Templates/BP_TaskManager.BP_TaskManager_C"))
      (Default|DoDamage _returnvalue (Variables|Default|GetActivateTime))
      (Utilities|FlowControl|Delay (Variables|/Game/Assets/Tasks/Templates/BP_TaskManager.BP_TaskManager_C|GetDamageDelay _returnvalue))
      (goto _label))))

(event Custom|SolveTask
  (Variables|Default|SetIsActive false)
  ;[1 1 1] Remove once compiling
  (Development|PrintString (Utilities|String|Append "Sovled - " (Utilities|GetClassDisplayName (Utilities|GetClass self)))))

(event Custom|SetupTask)

(fn ConstructionScript)
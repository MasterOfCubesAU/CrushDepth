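; Pressure destabilisation task Blueprint, solved when current pressure equals target pressure within a time limit.
; Setup draws two differing random pressures, shows them on text displays and starts a looping one-second timer.
; The timer counts elapsed time and calls SolveTask on an exact match before the limit; pressure adjustment happens outside this graph.
; Interaction blends the camera to the task, shows the cursor, ignores move/look input and sets player state InTask.
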(event EventInteraction
  (CallFunction|FocusonTask))

(event EventSetupTask
  (bind _returnvalue (CallFunction|GenerateFloat :!label _label))
  (bind _returnvalue_2 (CallFunction|GenerateFloat))
  (if (!= _returnvalue_2 _returnvalue)
    (bind _output_get (Variables|Default|SettargetPressure _returnvalue))
    (bind _output_get_2 (Variables|Default|SetCurrentPressure _returnvalue_2))
    (Rendering|Components|TextRender|SetText (Variables|Default|GetCurrVal) (Utilities|Text|ToText(Float) _output_get_2 "HalfToEven"))
    (Rendering|Components|TextRender|SetText (Variables|Default|GetTarVal) (Utilities|Text|ToText(Float) _output_get "HalfToEven"))
    (Utilities|Time|SetTimerbyFunctionName 0 "PressureWin" 1.0 true)
    (else
      (goto _label))))

(fn ConstructionScript
  (|CallParentFunction))

(fn PressureWin
  (Variables|Default|Settime (+ (Variables|Default|Gettime) 1.0))
  (if (< (Variables|Default|Gettime) 25.0)
    (if (== (Variables|Default|GetCurrentPressure) (Variables|Default|GettargetPressure))
      (CallFunction|SolveTask))))

(fn FocusonTask
  (CallFunction|IgnoreInput)
  (Game|Player|SetViewTargetwithBlend (Game|GetPlayerController 0) self 0.0 "VTBlend_Linear" 0.0 false)
  (bind _ascd_player_state (Utilities|Casting|CastToCD_PlayerState (Game|GetPlayerState 0)))
  (Class|CDPlayerState|SetPlayerState _ascd_player_state "InTask"))

(fn IgnoreInput
  (bind _returnvalue (Game|GetPlayerController 0))
  (Variables|/Script/Engine.PlayerController|SetbShowMouseCursor _returnvalue true)
  (Input|SetIgnoreMoveInput _returnvalue true)
  (Input|SetIgnoreLookInput _returnvalue true))

(fn GenerateFloat
  (bind _returnvalue (Math|Random|RandomFloatinRange 1e+03 1.5e+03))
  (return (- _returnvalue (Math|Float|%(Float) _returnvalue 5e+01))))
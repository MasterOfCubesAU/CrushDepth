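; BP_TaskManager runs a submarine dive session, activating tasks and tracking sub health, with debug keys to start dives or trigger a task.
; After a grace period, a Delay loop activates the single BP_TaskExample if idle, at randomized intervals that shorten as the dive progresses.
; DoDamage, meant for active tasks, adds (not subtracts) clamped time-scaled damage to Health.
; Health at zero or below ends the dive.
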(event Custom|Event_Destroyed
  ;[1 1 1] Gameover stuff
  (Variables|Default|SetInDive false)
  (Variables|Default|SetSubStartHealth 1000)
  (Development|PrintText "Sub Destroyed" true true "(R=0.000000,G=0.660000,B=1.000000,A=1.000000)" 5.0))

(event Custom|DiveStart
  (Development|PrintString "Dive started" true true "(R=0.000000,G=0.660000,B=1.000000,A=1.000000)" 5.0)
  (CallFunction|PrepareDive)
  (Utilities|FlowControl|Delay (Variables|Default|GetGracePeriodLength))
  (Development|PrintString "End Grace" true true "(R=0.000000,G=0.660000,B=1.000000,A=1.000000)" 5.0)
  ;[0.01938 0.01938 0.01938] Algo loop during dive
  (if (Variables|Default|GetInDive) :!label _label
    (CallFunction|PickTaskandActivate)
    (bind _taskdelay (CallFunction|GetTaskDelayTime))
    (Utilities|FlowControl|Delay _taskdelay)
    (goto _label)))

(event EventBeginPlay
  ;[1 1 1] Debug stuff
  (Input|EnableInput (Game|GetPlayerController 0))
  (CallFunction|PrepareGame))

(event Collision|EventActorBeginOverlap
  (params (OtherActor :type Actor%20Object%20Reference)))

(event EventTick
  (params (DeltaSeconds :type Float%20%28single-precision%29)))

(event Input|KeyboardEvents|1
  (params (Key :type Key%20Structure :default "None"))
  ;[1 1 1] Debug stuff
  (:Pressed
    (CallFunction|DiveStart)))

(event Input|KeyboardEvents|2
  (params (Key :type Key%20Structure :default "None"))
  (:Pressed
    (bind _returnvalue (Actor|GetActorOfClass "/Game/Assets/BP_TaskExample.BP_TaskExample_C"))
    (Default|EventActivate _returnvalue (Utilities|Time|GetGameTimeinSeconds))))

(fn ConstructionScript)

(fn PrepareGame
  (Variables|Default|SetDamageDelay 5.0)
  (Variables|Default|SetSubStartHealth 1000))

(fn PrepareDive
  (Variables|Default|SetDiveStartTime (Utilities|Time|GetGameTimeinSeconds))
  (Variables|Default|SetInDive true)
  (Variables|Default|SetHealth (Variables|Default|GetSubStartHealth)))

(fn GetTaskDelayTime
  (bind _returnvalue (Utilities|Time|GetGameTimeinSeconds))
  (bind _returnvalue_2 (Math|Random|RandomFloatinRange 0.9 1.1))
  (bind _divestarttime (Variables|Default|GetDiveStartTime))
  (bind _returnvalue_3 (- _returnvalue _divestarttime))
  (bind _returnvalue_4 (/ 1.5e+03 _returnvalue_3))
  (bind _returnvalue_5 (Math|Float|Clamp(Float) _returnvalue_4 5.0 3e+01))
  (bind _returnvalue_6 (* _returnvalue_5 _returnvalue_2))
  (Development|PrintString (Utilities|String|Append (Utilities|String|Append (Utilities|String|Append "Game time: " (Utilities|String|ToString(Float) _returnvalue)) " Task delay: ") (Utilities|String|ToString(Float) _returnvalue_6)) true true "(R=0.000000,G=0.660000,B=1.000000,A=1.000000)" 5.0)
  (return _returnvalue_6))

(fn PickTaskandActivate
  (if true
    (bind _returnvalue (Actor|GetActorOfClass "/Game/Assets/BP_TaskExample.BP_TaskExample_C"))
    (if (not (Variables|/Game/Assets/BP_TaskTemplate.BP_TaskTemplate_C|GetIsActive _returnvalue))
      (Default|EventActivate _returnvalue (Utilities|Time|GetGameTimeinSeconds)))))

(fn DoDamage
  (params (activateTime :type Float%20%28double-precision%29))
  (bind _damagetaken (CallFunction|CalculateDamage activateTime))
  (bind _output_get (Variables|Default|SetHealth (+ (Variables|Default|GetHealth) _damagetaken)))
  ;[1 1 1] Delete when final compiling
  (Development|PrintString (Utilities|String|BuildString(Integer) "Damaged by: " "" _damagetaken) true true "(R=0.000000,G=0.660000,B=1.000000,A=1.000000)" 5.0)
  (if (<= _output_get 0)
    (CallFunction|EventDestroyed)))

(fn CalculateDamage
  (params (TaskAppearTime :type Float%20%28double-precision%29))
  (return (Math|Integer|Clamp(Integer) (- (Math|Conversions|ToInteger(Byte) (Class|KismetMathLibrary|ToInt64(Float) (- (Utilities|Time|GetGameTimeinSeconds) TaskAppearTime))) 20) 0 50)))